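; Light actor Blueprint whose spotlight fades on and off with the game's darkness events.
; On BeginPlay it binds to the DarknessTickSubsystem's OnDarknessStart and OnDarknessStop delegates.
; Each event plays its own timeline, lerping SpotLight intensity between IntensityOn and IntensityOff.
; The construction script sets the spotlight to IntensityOn as its initial state.
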(event `self.ReceiveBeginPlay`
  (bind _returnvalue (subsystem `DarknessTickSubsystem`))
  (add `DarknessTickSubsystem.OnDarknessStop` _returnvalue (delegate `Turn on Lights`))
  (add `DarknessTickSubsystem.OnDarknessStart` _returnvalue (delegate `Turn off Lights`)))

(event `Turn off Lights`
  (bind (_direction _newtrack_0) (`Timeline|Timeline_0` :!via `PlayFromStart`)
    (:`Update`
      (`LightComponent.SetIntensity` (`self.SpotLight`) (`KismetMathLibrary.Lerp` (`self.IntensityOn`) (`self.IntensityOff`) _newtrack_0)))))

(event `Turn on Lights`
  (bind (_direction _newtrack_0) (`Timeline|Timeline` :!via `PlayFromStart`)
    (:`Update`
      (`LightComponent.SetIntensity` (`self.SpotLight`) (`KismetMathLibrary.Lerp` (`self.IntensityOff`) (`self.IntensityOn`) _newtrack_0)))))

(fn `UserConstructionScript`
  (`LightComponent.SetIntensity` (`self.SpotLight`) (`self.IntensityOn`)))