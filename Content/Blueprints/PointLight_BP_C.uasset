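; PointLight_BP is a point light Blueprint whose intensity can be faded between configurable on and off levels.
; The construction script calls its parent, then sets the light to IntensityOn.
; TurnOff and Turnon events lerp the intensity in opposite directions from a passed-in Alpha, leaving fade timing to the caller.
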(event `self.Turn Off`
  (params (Alpha :type "Float (double-precision)"))
  (`LightComponent.SetIntensity` (`self.PointLight`) (`KismetMathLibrary.Lerp` (`self.IntensityOn`) (`self.IntensityOff`) Alpha)))

(event `self.Turn on`
  (params (Alpha :type "Float (double-precision)"))
  (`LightComponent.SetIntensity` (`self.PointLight`) (`KismetMathLibrary.Lerp` (`self.IntensityOff`) (`self.IntensityOn`) Alpha)))

(fn `UserConstructionScript`
  (`parent.UserConstructionScript`)
  (`LightComponent.SetIntensity` (`self.PointLight`) (`self.IntensityOn`)))