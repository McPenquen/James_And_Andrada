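; GameManager Blueprint that switches all level lights in response to the game's darkness cycle.
; On BeginPlay it binds to DarknessTickSubsystem's stop and start events to turn lights on and off respectively.
; Each handler gathers every Light_BP actor and plays its own timeline, feeding the track value into each light's TurnOn on every update.
; Only turning on plays a 2D sound cue.
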(event `self.ReceiveBeginPlay`
  (bind _returnvalue (subsystem `DarknessTickSubsystem`))
  (add `DarknessTickSubsystem.OnDarknessStop` _returnvalue (delegate `Turn on all Lights`))
  (add `DarknessTickSubsystem.OnDarknessStart` _returnvalue (delegate `Turn off all Lights`)))

(event `Turn on all Lights`
  (`GameplayStatics.PlaySound2D` "/Game/Audio/LightOn_cue.LightOn_cue" 1.0 1.0 0.0 null null)
  (bind _outactors (`GameplayStatics.GetAllActorsOfClass` "/Game/Blueprints/Light_BP.Light_BP_C"))
  (bind (_direction _newtrack_0) (`Timeline|Timeline` :!via `PlayFromStart`)
    (:`Update`
      (for _array_element _outactors
        (`/Game/Blueprints/Light_BP.Turn on` _array_element _newtrack_0)))))

(event `Turn off all Lights`
  (bind _outactors (`GameplayStatics.GetAllActorsOfClass` "/Game/Blueprints/Light_BP.Light_BP_C"))
  (`|ExecutionSequence`
    (:`then_0`
      (bind (_direction _newtrack_0) (`Timeline|Timeline_0` :!via `PlayFromStart`)
        (:`Update`
          (for _array_element _outactors
            (`/Game/Blueprints/Light_BP.Turn on` _array_element _newtrack_0)))))))

(fn `UserConstructionScript`)