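; BlockingEnemy_BP is an enemy character that patrols a list of path stop actors and moves only during darkness.
; AIMoveTo drives a ping-pong patrol, pausing at each stop and advancing even when a move fails.
; DarknessTickSubsystem events toggle, after a short delay, its tick, walk speed and skeleton updates, freezing it when darkness stops.
; Hunt, give-up and run-speed values are initialized but unused in these graphs.
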(event `Move To Next Stop`
  (bind _pathstops (`self.PathStops`))
  ;[1 1 1] Movement
  (if (not (`KismetArrayLibrary.Array_IsEmpty` _pathstops))
    (`|AIMoveTo` self (`self.K2_GetActorLocation` (`|GetArrayItem` _pathstops (`self.CurrentPathSTopIndex`))) null 3.0
      (:`OnSuccess`
        _)
      (:`OnFail`
        _))
    (`KismetSystemLibrary.Delay` 2.0)
    (if (`self.IsIncrementing`)
      (if (< (+ (`self.CurrentPathSTopIndex`) 1) (`KismetArrayLibrary.Array_Length` (`self.PathStops`)))
        (set `self.CurrentPathSTopIndex` (+ (`self.CurrentPathSTopIndex`) 1))
        (else
          (set `self.IsIncrementing` false)
          (set `self.CurrentPathSTopIndex` (- (`self.CurrentPathSTopIndex`) 1))))
      (elif (>= (- (`self.CurrentPathSTopIndex`) 1) 0)
        (set `self.CurrentPathSTopIndex` (- (`self.CurrentPathSTopIndex`) 1))
        (else
          (set `self.IsIncrementing` true)
          (set `self.CurrentPathSTopIndex` (+ (`self.CurrentPathSTopIndex`) 1)))))
    (`self.Move To Next Stop`)))

(event `self.ReceiveBeginPlay`
  (bind _returnvalue (subsystem `DarknessTickSubsystem`))
  (bind _maxwalkspeed (`CharacterMovementComponent.MaxWalkSpeed` (`self.CharacterMovement`)))
  (set `self.PlayerChar` (`GameplayStatics.GetPlayerCharacter` 0))
  (set `self.MaxHuntLength` 5.0)
  (set `self.CurrentHuntLength` 0.0)
  (set `self.CurrentGivingUpTime` 0.0)
  ;[1 1 1] DarknessEvents
  (add `DarknessTickSubsystem.OnDarknessStart` _returnvalue (delegate `OnDarknessStart_Event`))
  (add `DarknessTickSubsystem.OnDarknessStop` _returnvalue (delegate `OnDarknessStop_Event`))
  (set `self.CurrentSpeed` _maxwalkspeed)
  (set `self.WalkSpeed` _maxwalkspeed)
  (set `self.RunSpeed` (+ _maxwalkspeed 200.0))
  (set `self.CurrentPathSTopIndex` 0)
  (`self.Move To Next Stop`))

(event `OnDarknessStart_Event`
  ;[1 1 1] DarknessEvents
  (`KismetSystemLibrary.Delay` 0.5)
  (`self.SetActorTickEnabled` true)
  (set `CharacterMovementComponent.MaxWalkSpeed` (`self.CurrentSpeed`) (`self.CharacterMovement`))
  (set `SkeletalMeshComponent.bNoSkeletonUpdate` false (`self.Mesh`)))

(event `OnDarknessStop_Event`
  ;[1 1 1] DarknessEvents
  (`KismetSystemLibrary.Delay` 0.5)
  (`self.SetActorTickEnabled` false)
  (set `CharacterMovementComponent.MaxWalkSpeed` 0.0 (`self.CharacterMovement`))
  (set `SkeletalMeshComponent.bNoSkeletonUpdate` true (`self.Mesh`)))

(fn `UserConstructionScript`)